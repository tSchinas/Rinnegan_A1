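; Player HUD Blueprint that sets up the player's reticle widget.
; On BeginPlay it creates WB_Reticle, caches the widget and its Reticle and ReticleCenter elements, and adds it to the viewport.
; Both reticle elements start collapsed, and the file has no logic to show them again.
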(event `self.ReceiveBeginPlay`
  (bind _returnvalue (`|CreateWidget` "/Game/UI/WB_Reticle.WB_Reticle_C"))
  (bind _output_get (set `self.WidgetRef` _returnvalue))
  (set `self.Reticle` (`/Game/UI/WB_Reticle.Reticle` _output_get))
  (set `self.ReticleCenter` (`/Game/UI/WB_Reticle.ReticleCenter` _output_get))
  (`UserWidget.AddToViewport` _output_get 0)
  (`Widget.SetVisibility` (`self.Reticle`) "Collapsed")
  (`Widget.SetVisibility` (`self.ReticleCenter`) "Collapsed"))

(fn `UserConstructionScript`)