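; Interaction component for BP_ThirdPersonCharacter that finds the interactive actor the follow camera is aimed at.
; Each tick it clears the target, runs a debug-drawn multi line trace forward from the camera, and scans hits by distance.
; A hit closer than any before it becomes CurrentTarget if it casts to BP_InteractiveActor.
; Interact calls InteractMessage on that target when it is valid.
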(event `self.ReceiveBeginPlay`
  (bind _asbp_third_person_character (cast `/Game/ThirdPerson/Blueprints/BP_ThirdPersonCharacter` (`self.GetOwner`)))
  (set `self.As BP Third Person Character` _asbp_third_person_character))

(event `self.ReceiveTick`
  (params (DeltaSeconds :type "Float (single-precision)"))
  (bind _as_bp_third_person_character (`self.As BP Third Person Character`))
  (bind _followcamera (`/Game/ThirdPerson/Blueprints/BP_ThirdPersonCharacter.FollowCamera` _as_bp_third_person_character))
  (bind _returnvalue (`SceneComponent.K2_GetComponentLocation` _followcamera))
  (set `self.CurrentTarget` null)
  (bind _outhits (`KismetSystemLibrary.LineTraceMulti` _returnvalue (+ _returnvalue (* (`SceneComponent.GetForwardVector` _followcamera) 1e+18)) "TraceTypeQuery3" false (`|MakeArray` _as_bp_third_person_character :!type "Actor Object Reference") "ForOneFrame"))
  (bind _output_get (set `self.ClosestDistance` 1e+18))
  (for _array_element _outhits
    (bind _returnvalue_2 (`KismetMathLibrary.Vector_Distance` _returnvalue (`.Location` (`GameplayStatics.BreakHitResult` _array_element))))
    (`/Engine/EditorBlueprintResources/StandardMacros.CompareFloat` _returnvalue_2 _output_get
      (:`<`
        (set `self.ClosestDistance` _returnvalue_2)
        (bind _asbp_interactive_actor (cast `/Game/BP_InteractiveActor` (`.HitActor` (`GameplayStatics.BreakHitResult` _array_element))))
        (set `self.CurrentTarget` _asbp_interactive_actor)))))

(fn `Interact`
  (bind _currenttarget (`self.CurrentTarget`))
  (`/Engine/EditorBlueprintResources/StandardMacros.IsValid` _currenttarget
    (:`Is Valid`
      (message `/Game/BI_Interactable.Interact` _currenttarget))))